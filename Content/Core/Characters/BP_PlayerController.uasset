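; BP_PlayerController is a player controller that toggles the game's pause state and pause menu from the Pause input action.
; Pausing creates a new UWB_PauseMenu widget, adds it to the viewport, pauses the game and shows the mouse cursor.
; Pressing Pause while the game is paused removes the stored widget, unpauses and hides the cursor.
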(event Input|ActionEvents|InputActionPause
  (params (Key :type Key%20Structure :default "None"))
  (:Pressed
    (if (Game|IsGamePaused)
      (Widget|RemovefromParent (Variables|Default|GetPauseMenu))
      (Game|SetGamePaused false)
      (Variables|Default|SetbShowMouseCursor false)
      (else
        (bind _returnvalue (UserInterface|CreateWidget "/Game/Core/UI/UWB_PauseMenu.UWB_PauseMenu_C"))
        (bind _output_get (Variables|Default|SetPauseMenu _returnvalue))
        (UserInterface|Viewport|AddtoViewport _output_get 0)
        (Game|SetGamePaused true)
        (Variables|Default|SetbShowMouseCursor true)))))

(fn ConstructionScript)